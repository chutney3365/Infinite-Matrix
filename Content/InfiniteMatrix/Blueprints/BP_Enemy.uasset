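; BP_Enemy is an enemy actor that damages the player on contact and awards score when shot.
; Its box overlap either decrements player health, triggering death and the restart display at exactly zero, or handles a BP_Projectile hit by raising score, updating the HUD and destroying the projectile.
; The enemy destroys itself on either hit, or when Tick finds the player's X location exceeds its own.
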(event OnComponentBeginOverlap(Box)
  (params (OverlappedComponent :type Primitive%20Component%20Object%20Reference) (OtherActor :type Actor%20Object%20Reference) (OtherComp :type Primitive%20Component%20Object%20Reference) (OtherBodyIndex :type Integer) (bFromSweep :type Boolean) (SweepResult :type Hit%20Result%20Structure%20%28by%20ref%29))
  (bind _asbp_player (Utilities|Casting|CastToBP_Player OtherActor)
    (:then
      (bind _result (Math|Float|DecrementFloat (Variables|/Game/InfiniteMatrix/Blueprints/BP_Player.BP_Player_C|GetPlayerHealth _asbp_player))
        (:%20%20
          (bind _output_get (Variables|/Game/InfiniteMatrix/Blueprints/BP_Player.BP_Player_C|SetPlayerHealth _asbp_player _result))
          (Actor|DestroyActor)
          (if (== _output_get 0.0)
            (Variables|/Game/InfiniteMatrix/Blueprints/BP_Player.BP_Player_C|SetIsDead _asbp_player true)
            (Default|DisplayRestart _asbp_player)))))
    (:CastFailed
      (bind _asbp_projectile (Utilities|Casting|CastToBP_Projectile OtherActor))
      (bind _returnvalue (Actor|GetActorOfClass "/Game/InfiniteMatrix/Blueprints/BP_Player.BP_Player_C"))
      (bind _result_2 (Math|Integer|IncrementInt (Variables|/Game/InfiniteMatrix/Blueprints/BP_Player.BP_Player_C|GetScore _returnvalue))
        (:%20%20
          (bind _output_get_2 (Variables|/Game/InfiniteMatrix/Blueprints/BP_Player.BP_Player_C|SetScore _returnvalue _result_2))
          (Default|UpdateScoreDisplay (Variables|/Game/InfiniteMatrix/Blueprints/BP_Player.BP_Player_C|GetHUD_HealthBar _returnvalue) _output_get_2)
          (Actor|DestroyActor)
          (Actor|DestroyActor _asbp_projectile))))))

(event EventBeginPlay)

(event Collision|EventActorBeginOverlap
  (params (OtherActor :type Actor%20Object%20Reference)))

(event EventTick
  (params (DeltaSeconds :type Float%20%28single-precision%29))
  (bind _returnvalue (Actor|GetActorOfClass "/Game/InfiniteMatrix/Blueprints/BP_Player.BP_Player_C"))
  (if (> (.x (Transformation|GetActorLocation _returnvalue)) (.x (Transformation|GetActorLocation)))
    (Actor|DestroyActor)))

(fn ConstructionScript)