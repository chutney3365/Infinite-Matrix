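; BP_HealthPack is a health pickup actor that raises the player's health on contact.
; Its Box overlap increments BP_Player's PlayerHealth up to a cap and destroys the pack, while an overlapping BP_Projectile is destroyed and leaves the pack intact.
; Tick looks up BP_Player by class every frame and destroys the pack once the player's X position exceeds its own.
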(event OnComponentBeginOverlap(Box)
  (params (OverlappedComponent :type Primitive%20Component%20Object%20Reference) (OtherActor :type Actor%20Object%20Reference) (OtherComp :type Primitive%20Component%20Object%20Reference) (OtherBodyIndex :type Integer) (bFromSweep :type Boolean) (SweepResult :type Hit%20Result%20Structure%20%28by%20ref%29))
  (bind _asbp_player (Utilities|Casting|CastToBP_Player OtherActor)
    (:then
      (bind _result (Math|Float|IncrementFloat (Variables|/Game/InfiniteMatrix/Blueprints/BP_Player.BP_Player_C|GetPlayerHealth _asbp_player))
        (:%20%20
          (Variables|/Game/InfiniteMatrix/Blueprints/BP_Player.BP_Player_C|SetPlayerHealth _asbp_player (Math|Float|Min(Float) _result 1e+01))
          (Actor|DestroyActor))))
    (:CastFailed
      (bind _asbp_projectile (Utilities|Casting|CastToBP_Projectile OtherActor))
      (Actor|DestroyActor _asbp_projectile))))

(event EventBeginPlay)

(event Collision|EventActorBeginOverlap
  (params (OtherActor :type Actor%20Object%20Reference)))

(event EventTick
  (params (DeltaSeconds :type Float%20%28single-precision%29))
  (bind _returnvalue (Actor|GetActorOfClass "/Game/InfiniteMatrix/Blueprints/BP_Player.BP_Player_C"))
  (if (> (.x (Transformation|GetActorLocation _returnvalue)) (.x (Transformation|GetActorLocation)))
    (Actor|DestroyActor)))

(fn ConstructionScript)